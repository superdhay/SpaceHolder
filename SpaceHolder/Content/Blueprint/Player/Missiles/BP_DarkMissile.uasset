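; BP_DarkMissile is a missile actor that damages player ships on overlap.
; On BeginPlay its StaticMesh ignores the owner when moving, and the missile destroys itself once MissileDuration elapses.
; Overlaps with the owner are skipped; any other overlap destroys the missile, calling TakeDamage first if the actor is a BP_PlayerPawn.
; Debug prints report what it hit, and the graph holds no movement logic.
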(event OnComponentBeginOverlap(StaticMesh)
  (params (OverlappedComponent :type Primitive%20Component%20Object%20Reference) (OtherActor :type Actor%20Object%20Reference) (OtherComp :type Primitive%20Component%20Object%20Reference) (OtherBodyIndex :type Integer) (bFromSweep :type Boolean) (SweepResult :type Hit%20Result%20Structure%20%28by%20ref%29))
  ;[1 1 1] Missile overlap consequences
  (if (!= (Components|GetOwner) OtherActor)
    (bind _asbp_player_pawn (Utilities|Casting|CastToBP_PlayerPawn OtherActor)
      (:then
        ;;[1 1 1] Hit ennemy ship
        (Development|PrintString "Touched player")
        (Default|TakeDamage _asbp_player_pawn true))
      (:CastFailed
        ;;[1 1 1] Hit something else
        (Development|PrintString (Utilities|GetDisplayName OtherActor))
        (Development|PrintString "Touched Something Else")))
    (Actor|DestroyActor)))

(event EventBeginPlay
  (Collision|IgnoreActorwhenMoving (Variables|Default|GetStaticMesh) (Components|GetOwner) true)
  (Utilities|FlowControl|Delay (Variables|Default|GetMissileDuration))
  (Actor|DestroyActor))

(fn ConstructionScript)