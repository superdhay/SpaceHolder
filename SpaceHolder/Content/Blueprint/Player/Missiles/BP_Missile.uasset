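; BP_Missile is a player-fired projectile with a light or dark mode that damages other player ships of the same mode.
; On BeginPlay it copies the owner's mode, switches from green to red material if dark, ignores the owner when moving and expires after MissileDuration.
; On overlap it damages and destroys itself on same-mode ships, passes through opposite-mode ships and destroys itself on other non-owner actors.
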(event OnComponentBeginOverlap(StaticMesh)
  (params (OverlappedComponent :type Primitive%20Component%20Object%20Reference) (OtherActor :type Actor%20Object%20Reference) (OtherComp :type Primitive%20Component%20Object%20Reference) (OtherBodyIndex :type Integer) (bFromSweep :type Boolean) (SweepResult :type Hit%20Result%20Structure%20%28by%20ref%29))
  ;[1 1 1] Missiles overlap event consequences
  (if (!= (Components|GetOwner) OtherActor)
    (bind _asbp_player_pawn (Utilities|Casting|CastToBP_PlayerPawn OtherActor)
      (:then
        ;;[1 1 1] Hit ennemy ship
        (Development|PrintString "Touched player")
        (if (Math|Boolean|Equal(Boolean) (Variables|Default|GetbIsDarkMode?) (Variables|/Game/Blueprint/Player/BP_PlayerPawn.BP_PlayerPawn_C|GetbIsDarkMode? _asbp_player_pawn))
          (Default|TakeDamage _asbp_player_pawn false)
          (Actor|DestroyActor :!label _label)))
      (:CastFailed
        ;;[1 1 1] Hit something else
        (Development|PrintString (Utilities|GetDisplayName OtherActor))
        (Development|PrintString "Touched Something Else")
        (goto _label)))))

(event EventBeginPlay
  (bind _output_get (Variables|Default|SetbIsDarkMode? (Variables|/Game/Blueprint/Player/BP_PlayerPawn.BP_PlayerPawn_C|GetbIsDarkMode? (.AsBP%20Player%20Pawn (Utilities|Casting|CastToBP_PlayerPawn (Components|GetOwner))))))
  (if _output_get
    (Rendering|Material|SetMaterial (Variables|Default|GetStaticMesh) 0 "/Engine/EngineDebugMaterials/VertexColorViewMode_RedOnly.VertexColorViewMode_RedOnly"))
  (Collision|IgnoreActorwhenMoving (Variables|Default|GetStaticMesh) (Components|GetOwner) true)
  (Utilities|FlowControl|Delay (Variables|Default|GetMissileDuration))
  (Actor|DestroyActor))

(fn ConstructionScript
  (Rendering|Material|CreateDynamicMaterialInstance (Variables|Default|GetStaticMesh) 0 "/Engine/EngineDebugMaterials/VertexColorViewMode_GreenOnly.VertexColorViewMode_GreenOnly" "None" :!class /Script/Engine.PrimitiveComponent))