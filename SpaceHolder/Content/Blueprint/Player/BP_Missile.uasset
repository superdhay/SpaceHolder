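; BP_Missile is a player missile actor that flies along the X axis when launched, then destroys itself.
; LaunchMissile plays the MissileMovement timeline, which lerps the Missile component's world X toward MaxMissileRange without sweeping.
; The start X and fixed Y and Z of that world location come from the component's world scale, not its position.
; The construction script applies NewMaterial to the Missile component.
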(event Custom|LaunchMissile
  (bind _missile (Variables|Default|GetMissile))
  (bind _returnvalue (Transformation|GetWorldScale _missile))
  (bind (_x _y _z) (Math|Vector|BreakVector _returnvalue))
  ;[1 1 1] Missile movement when fired
  (bind _alpha (Timeline|MissileMovement Play)
    (:Update
      (Transformation|SetWorldLocation (Variables|Default|GetMissile) (Math|Vector|MakeVector (Math|Float|Lerp _x (Variables|Default|GetMaxMissileRange) _alpha) _y _z) false false))
    (:Finished
      ;[1 1 1] Destroy it after finishing its movement
      (Actor|DestroyActor))))

(fn ConstructionScript
  (Rendering|Material|SetMaterial (Variables|Default|GetMissile) 0 (Variables|Default|GetNew%20Material)))