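; Player ship pawn for a shooter, handling movement, lives, firing, power-ups, pausing and a dark/light mode toggle.
; Damage costs a life and starts a blinking invincibility timeline, or ends the game through BP_GM at zero.
; Held fire re-calls Shoot at the fire rate, choosing timed triple, timed banana or simple missiles.
; Mode toggling drives dynamic hull and paint materials, and a broken shield destroys nearby actors via sphere trace.
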(event Custom|TakeDamage
  ;[1 1 1] Player take damage event
  (if (not (Variables|Default|GetbIsInvincible?))
    (Variables|Default|SetbIsInvincible? true)
    (bind _output_get (Variables|ShipStats|SetLifePoints (- (Variables|ShipStats|GetLifePoints) 1)))
    (if (<= _output_get 0)
      (Default|EndOfGame (.AsBP%20GM (Utilities|Casting|CastToBP_GM (Game|GetGameMode))))
      (else
        (Default|TakeDamage (Variables|Default|GetLifePointsUI))
        (Timeline|Invicibility PlayFromStart
          (:Finished
            (Rendering|SetVisibility (Variables|Default|GetSkeletalMesh) true false)
            (Variables|Default|SetbIsInvincible? false))
          (:Visibility
            (Rendering|ToggleVisibility (Variables|Default|GetSkeletalMesh) false)))))))

(event Custom|Shoot
  ;[1 1 1] Shoot action
  (if (Variables|ShipFireing|GetbIsFiring?)
    (if (Variables|ShipFireing|GetbTripleShot)
      (CallFunction|TripleShot)
      (elif (Variables|ShipFireing|GetbIsBananaShot?)
        (CallFunction|BananaShot)
        (else
          (CallFunction|SimpleShot))))
    (Utilities|FlowControl|Delay (/ 1.0 (Variables|ShipFireing|GetRofPerSec)))
    (CallFunction|Shoot)))

(event Custom|TripleShot
  (bind _returnvalue (Transformation|GetActorTransform))
  (bind _self self)
  (bind _tripleshotangle (Variables|ShipFireing|GetTripleShotAngle))
  (bind (_location _rotation) (Math|Transform|BreakTransform _returnvalue))
  (bind (_roll _pitch _yaw) (Math|Rotator|BreakRotator _rotation))
  ;[1 1 1] Triple Shot
  (CallFunction|SimpleShot)
  ;;[1 1 1] Angled Shots
  (Game|SpawnActorfromClass "/Game/Blueprint/Player/Missiles/BP_Missile.BP_Missile_C" (Math|Transform|MakeTransform _location (Math|Rotator|MakeRotator _roll _pitch (+ _yaw _tripleshotangle))) "Undefined" _self 0)
  (Game|SpawnActorfromClass "/Game/Blueprint/Player/Missiles/BP_Missile.BP_Missile_C" (Math|Transform|MakeTransform _location (Math|Rotator|MakeRotator _roll _pitch (- _yaw _tripleshotangle))) "Undefined" _self 0))

(event Custom|SimpleShot
  ;[1 1 1] Simple Shot
  (Game|SpawnActorfromClass "/Game/Blueprint/Player/Missiles/BP_Missile.BP_Missile_C" (Transformation|GetActorTransform) "Undefined" self 0))

(event Custom|ShieldHit
  (bind _returnvalue (Transformation|GetActorLocation))
  (bind _shield (Variables|Default|GetShield))
  (Development|PrintString "ShieldIsBroken")
  (Collision|SetCollisionEnabled _shield "NoCollision")
  (Rendering|SetVisibility _shield false false)
  (bind _outhits (Collision|MultiSphereTraceForObjects _returnvalue _returnvalue (Variables|ShipFireing|GetDestroyRadius) (Utilities|Array|MakeArray "ObjectTypeQuery7") false 0 "Persistent"))
  (for _array_element _outhits
    (Utilities|IsValid (.HitActor (Collision|BreakHitResult _array_element))
      (:Is%20Valid
        (Actor|DestroyActor (.HitActor (Collision|BreakHitResult _array_element)))))))

(event Custom|GetShield
  (bind _shield (Variables|Default|GetShield))
  (Collision|SetCollisionEnabled _shield "QueryAndPhysics")
  (Rendering|SetVisibility _shield true false))

(event Custom|EnableTripleShot
  (Variables|ShipFireing|SetbTripleShot true)
  (Utilities|FlowControl|RetriggerableDelay (Variables|ShipFireing|GetTripleShotDuration))
  (Variables|ShipFireing|SetbTripleShot false))

(event Custom|BananaShot
  (Game|SpawnActorfromClass "/Game/Blueprint/Player/Missiles/BP_BananaMissile.BP_BananaMissile_C" (Transformation|GetActorTransform) "Undefined" self 0))

(event Custom|EnableBananaShot
  (Variables|ShipFireing|SetbIsBananaShot? true)
  (Utilities|FlowControl|RetriggerableDelay (Variables|ShipFireing|GetBanananDuration))
  (Variables|ShipFireing|SetbIsBananaShot? false))

(event EventBeginPlay
  (Components|Timeline|SetPlayRate (Variables|Default|GetInvicibility) (/ 1.0 (Variables|ShipStats|GetInvicibilityDuration))))

(event Input|ActionEvents|InputActionShoot
  (params (Key :type Key%20Structure :default "None"))
  ;[1 1 1] Player shoot action
  (:Pressed
    (Variables|ShipFireing|SetbIsFiring? true)
    (CallFunction|Shoot))
  (:Released
    (Variables|ShipFireing|SetbIsFiring? false)))

(event Input|ActionEvents|InputActionChangeMode
  (params (Key :type Key%20Structure :default "None"))
  (bind _mihull (Variables|Default|GetMIHull))
  (bind _mipaint (Variables|Default|GetMIPaint))
  ;[1 1 1] Toggle to the other mod
  (:Pressed
    ;;[0 0 0] Set gun fire type
    (bind _output_get (Variables|ShipStats|SetbIsDarkMode? (not (Variables|ShipStats|GetbIsDarkMode?))))
    ;;[0 0 0] Set material type
    (if _output_get
      (Rendering|Material|SetScalarParameterValue _mihull "Swap_Intensity" 0.0 :!class /Script/Engine.MaterialInstanceDynamic)
      (Rendering|Material|SetScalarParameterValue _mipaint "Swap_Intensity" 0.0 :!class /Script/Engine.MaterialInstanceDynamic)
      (else
        (Rendering|Material|SetScalarParameterValue _mihull "Swap_Intensity" 1.0 :!class /Script/Engine.MaterialInstanceDynamic)
        (Rendering|Material|SetScalarParameterValue _mipaint "Swap_Intensity" 1.0 :!class /Script/Engine.MaterialInstanceDynamic)))))

(event Input|ActionEvents|InputActionPause
  (params (Key :type Key%20Structure :default "None"))
  ;[1 1 1] Pause Menu
  (:Pressed
    (bind _returnvalue (UserInterface|CreateWidget "/Game/UI/W_PauseMenu.W_PauseMenu_C"))
    (bind _output_get (Variables|Default|SetPauseUI _returnvalue))
    (UserInterface|Viewport|AddtoViewport _output_get 0)
    (Game|SetGamePaused true)))

(event Input|AxisEvents|InputAxisMovementVertical
  (params (AxisValue :type Float%20%28single-precision%29))
  ;[1 1 1] Player movements
  (Pawn|Input|AddMovementInput (Math|Vector|MakeVector (stale Input|AxisEvents|InputAxisMovementHorizontal AxisValue) (* AxisValue -1.0) 0.0) (Variables|ShipMovement|GetMovementScale) false))

(event Input|AxisEvents|InputAxisMovementHorizontal
  (params (AxisValue :type Float%20%28single-precision%29))
  ;[1 1 1] Player movements
  (Pawn|Input|AddMovementInput (Math|Vector|MakeVector AxisValue (* (stale Input|AxisEvents|InputAxisMovementVertical AxisValue) -1.0) 0.0) (Variables|ShipMovement|GetMovementScale) false))

(fn ConstructionScript
  (Utilities|FlowControl|Sequence
    (:then_1
      ;[1 1 1] Set ship dynamic material for changing mode
      (bind _returnvalue (Rendering|Material|CreateDynamicMaterialInstance (Variables|Default|GetSkeletalMesh) 0 "/Game/Materials/M_Ship_Hull.M_Ship_Hull" "None" :!class /Script/Engine.PrimitiveComponent))
      (Variables|Default|SetMIHull _returnvalue)
      (bind _returnvalue_2 (Rendering|Material|CreateDynamicMaterialInstance (Variables|Default|GetSkeletalMesh) 1 "/Game/Materials/M_Ship_Paint.M_Ship_Paint" "None" :!class /Script/Engine.PrimitiveComponent))
      (Variables|Default|SetMIPaint _returnvalue_2))
    (:then_2
      (Variables|ShipStats|SetbIsDarkMode? false))))