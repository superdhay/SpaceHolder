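; BP_MultiLocal sets up a two-player local multiplayer session that shares one fixed camera.
; On BeginPlay it creates two local players, spawns a BP_PlayerPawn at each of two placeholder box components, destroys the boxes, and has each controller possess its pawn.
; Both controllers' view targets switch to this actor.
; A single W_PlayersLifePoints widget is handed to both pawns and added to the viewport.
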(event Custom|CreateID
  ;[1 1 1] Create player id
  (Class|GameplayStatics|CreatePlayer 0)
  (Variables|Default|SetPCPlayer1 (Game|GetPlayerController 0))
  (Class|GameplayStatics|CreatePlayer 1)
  (Variables|Default|SetPCPlayer2 (Game|GetPlayerController 1))
  (CallFunction|CreatePawn))

(event Custom|CreatePawn
  ;[1 1 1] Create player pawn
  (bind _returnvalue (Game|SpawnActorfromClass "/Game/Blueprint/Player/BP_PlayerPawn.BP_PlayerPawn_C" (Transformation|GetWorldTransform (Variables|Default|GetBox)) "Undefined" 0 0))
  (Variables|Default|SetActorPlayer1 _returnvalue)
  (Components|DestroyComponent (Variables|Default|GetBox))
  (bind _returnvalue_2 (Game|SpawnActorfromClass "/Game/Blueprint/Player/BP_PlayerPawn.BP_PlayerPawn_C" (Transformation|GetWorldTransform (Variables|Default|GetBox1)) "Undefined" 0 0))
  (Variables|Default|SetActorPlayer2 _returnvalue_2)
  (Components|DestroyComponent (Variables|Default|GetBox1))
  (CallFunction|PossessPlayers))

(event Custom|PossessPlayers
  (bind _pcplayer2 (Variables|Default|GetPCPlayer2))
  ;[1 1 1] Possess player by user
  (Pawn|Possess (Variables|Default|GetPCPlayer1) (Variables|Default|GetActorPlayer1))
  (CallFunction|SwitchCameraFixe)
  (Pawn|Possess _pcplayer2 (Variables|Default|GetActorPlayer2))
  (Game|Player|SetViewTargetwithBlend _pcplayer2 self 0.0 "VTBlend_Linear" 0.0 false)
  (CallFunction|SwitchCameraFixe)
  (CallFunction|AddUI))

(event Custom|SwitchCameraFixe
  ;[1 1 1] Set camera
  (Game|Player|SetViewTargetwithBlend (Game|GetPlayerController 0) self 0.0 "VTBlend_Linear" 0.0 false))

(event Custom|AddUI
  ;[1 1 1] Add UI to player
  (bind _returnvalue (UserInterface|CreateWidget "/Game/UI/W_PlayersLifePoints.W_PlayersLifePoints_C"))
  (bind _output_get (Variables|/Game/Blueprint/Player/BP_PlayerPawn.BP_PlayerPawn_C|SetLifePointsUI (Variables|Default|GetActorPlayer1) _returnvalue))
  (bind _output_get_2 (Variables|/Game/Blueprint/Player/BP_PlayerPawn.BP_PlayerPawn_C|SetLifePointsUI (Variables|Default|GetActorPlayer2) _output_get))
  (UserInterface|Viewport|AddtoViewport _output_get_2 0))

(event EventBeginPlay
  ;[1 1 1] Call event to create player id
  (CallFunction|CreateID))

(fn ConstructionScript)