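; BP_PlayerControler is the player controller that routes menu navigation input to the pause menu.
; On Confirm, Up or Down presses, it casts the controlled pawn to BP_PlayerPawn and calls the matching Select, Up or Down function on that pawn's PauseUI.
; Each call runs only while PauseUI is valid, and the controller holds no other logic.
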(event Input|ActionEvents|InputActionDown
  (params (Key :type Key%20Structure :default "None"))
  (bind _returnvalue (Pawn|GetControlledPawn))
  (bind _asbp_player_pawn (Utilities|Casting|CastToBP_PlayerPawn _returnvalue))
  (bind _pauseui (Variables|/Game/Blueprint/Player/BP_PlayerPawn.BP_PlayerPawn_C|GetPauseUI _asbp_player_pawn))
  (:Pressed
    (Utilities|IsValid _pauseui
      (:Is%20Valid
        (Default|Down _pauseui)))))

(event Input|ActionEvents|InputActionUp
  (params (Key :type Key%20Structure :default "None"))
  (bind _returnvalue (Pawn|GetControlledPawn))
  (bind _asbp_player_pawn (Utilities|Casting|CastToBP_PlayerPawn _returnvalue))
  (bind _pauseui (Variables|/Game/Blueprint/Player/BP_PlayerPawn.BP_PlayerPawn_C|GetPauseUI _asbp_player_pawn))
  (:Pressed
    (Utilities|IsValid _pauseui
      (:Is%20Valid
        (Default|Up _pauseui)))))

(event Input|ActionEvents|InputActionConfirm
  (params (Key :type Key%20Structure :default "None"))
  (bind _returnvalue (Pawn|GetControlledPawn))
  (bind _asbp_player_pawn (Utilities|Casting|CastToBP_PlayerPawn _returnvalue))
  (bind _pauseui (Variables|/Game/Blueprint/Player/BP_PlayerPawn.BP_PlayerPawn_C|GetPauseUI _asbp_player_pawn))
  (:Pressed
    (Utilities|IsValid _pauseui
      (:Is%20Valid
        (Default|Select _pauseui)))))

(fn ConstructionScript)