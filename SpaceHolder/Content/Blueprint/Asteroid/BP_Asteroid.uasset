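; BP_Asteroid is an asteroid actor that moves its mesh along the Z axis and can take a random look.
; On BeginPlay, the AsteroidMovement timeline lerps the mesh's current world Z toward MaxValue each update, keeping X and Y.
; Because the lerp restarts from the current position, the motion compounds rather than following the alpha curve directly.
; A separate SetAsteroid event assigns a random static mesh from the Asteroids array.
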(event Custom|SetAsteroid
  (bind _asteroids (Variables|Default|GetAsteroids))
  ;[1 1 1] Set list of static mesh
  (Components|StaticMesh|SetStaticMesh (Variables|Default|GetAsteroid) (Utilities|Array|Get(acopy) _asteroids (Math|Random|RandomIntegerinRange 0 (- (Utilities|Array|Length _asteroids) 1)))))

(event EventBeginPlay
  (bind _asteroid (Variables|Default|GetAsteroid))
  (bind _returnvalue (Transformation|GetWorldLocation _asteroid))
  (bind (_x _y _z) (Math|Vector|BreakVector _returnvalue))
  ;[1 1 1] Asteroid movement
  (bind _alpha (Timeline|AsteroidMovement Play)
    (:Update
      (Transformation|SetWorldLocation (Variables|Default|GetAsteroid) (Math|Vector|MakeVector _x _y (Math|Float|Lerp _z (Variables|Default|GetMaxValue) _alpha)) false false))))

(fn ConstructionScript)