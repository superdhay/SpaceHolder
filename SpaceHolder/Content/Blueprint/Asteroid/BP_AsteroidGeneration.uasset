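; BP_AsteroidGeneration is an asteroid spawner that also removes asteroids reaching its collision volume.
; From BeginPlay, an endless Delay loop spawns one BP_Asteroid and calls SetAsteroid on it, then waits a random whole number of seconds.
; A spawn-transform graph builds the location from the Generator component's position with an X offset.
; The Collision overlap event destroys any overlapping BP_Asteroid.
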(event OnComponentBeginOverlap(Collision)
  (params (OverlappedComponent :type Primitive%20Component%20Object%20Reference) (OtherActor :type Actor%20Object%20Reference) (OtherComp :type Primitive%20Component%20Object%20Reference) (OtherBodyIndex :type Integer) (bFromSweep :type Boolean) (SweepResult :type Hit%20Result%20Structure%20%28by%20ref%29))
  (bind (_asbp_asteroid _bsuccess) (Utilities|Casting|CastToBP_Asteroid OtherActor))
  ;[1 1 1] Destroy asteroid when there are on the collision box
  (if _bsuccess
    (Actor|DestroyActor _asbp_asteroid)))

(event EventBeginPlay
  ;[1 1 1] Generate BP_Asteroid at random time
  (for _index (range 0 0) :!label _label
    (bind _returnvalue (Game|SpawnActorfromClass "/Game/Blueprint/Asteroid/BP_Asteroid.BP_Asteroid_C" (|SpawnBP_Asteroidtransform) "Undefined" 0 0))
    (Default|SetAsteroid _returnvalue))
  (Utilities|FlowControl|Delay (Math|Conversions|ToFloat(Integer) (Math|Random|RandomIntegerinRange 1 3)))
  (goto _label))

(fn ConstructionScript)